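; BP_Enemy is a basic enemy that chases the player and dies as a ragdoll.
; Every Tick issues an AI MoveTo toward the player character.
; KillMe turns on mesh physics and disables capsule collision, then after a short delay makes the mesh ignore all collision and sets a lifespan so the body is removed.
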(event `self.ReceiveTick`
  (params (DeltaSeconds :type "Float (single-precision)"))
  ;[1 1 1] AI move to player position
  (`|AIMoveTo` self (0.0 0.0 0.0) (`GameplayStatics.GetPlayerCharacter` 0) 100.0))

(event `Kill Me`
  (`PrimitiveComponent.SetSimulatePhysics` (`self.Mesh`) true)
  (`PrimitiveComponent.SetCollisionEnabled` (`self.Mesh`) "PhysicsOnly")
  (`PrimitiveComponent.SetCollisionEnabled` (`self.CapsuleComponent`) "NoCollision")
  (`KismetSystemLibrary.Delay` 2.0)
  (`PrimitiveComponent.SetCollisionResponseToAllChannels` (`self.Mesh`) "ECR_Ignore")
  (`self.SetLifeSpan` 3.0))

(fn `UserConstructionScript`)
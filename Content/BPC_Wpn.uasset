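; BPC_Wpn is a weapon component that periodically kills every enemy within a radius of its owner, with no input trigger.
; Tick counts Cooldown down by delta time, then resets it to CooldownMax and fires.
; Each shot runs a sphere overlap for BP_Enemy pawns at the owner's location and calls KillMe on each.
; A briefly drawn red debug sphere is the only visual for the attack.
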(event `self.ReceiveTick`
  (params (DeltaSeconds :type "Float (single-precision)"))
  (bind _returnvalue (`Actor.K2_GetActorLocation` (`self.GetOwner`)))
  (if (> (`self.Cooldown`) 0.0)
    (set `self.Cooldown` (- (`self.Cooldown`) (`GameplayStatics.GetWorldDeltaSeconds`)))
    (else
      (`KismetSystemLibrary.DrawDebugSphere` _returnvalue (`self.Radius`) 12 (struct :`R` 1.0 :`A` 1.0) 0.5 2.0)
      (set `self.Cooldown` (`self.Cooldown Max`))
      (bind _outactors (`KismetSystemLibrary.SphereOverlapActors` _returnvalue (`self.Radius`) (`|MakeArray` "ObjectTypeQuery3" :!type "EObjectTypeQuery Enum") "/Game/BP_Enemy.BP_Enemy_C"))
      (for _array_element _outactors
        (bind _asbp_enemy (cast `/Game/BP_Enemy` _array_element))
        (`/Game/BP_Enemy.Kill Me` _asbp_enemy)))))